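; Drone motor component that acts as a single thrust point on the physics body of its owning actor.
; It caches the owner's root primitive at BeginPlay and accumulates thrust through Add Force.
; Apply Force pushes the body along the motor's up vector at the motor's location, producing off-center rotation, then clears the total.
; Add Torque immediately applies torque about world Z, and Reset discards pending thrust.
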(event `self.ReceiveBeginPlay`
  (bind _asprimitive_component (cast `PrimitiveComponent` (`Actor.RootComponent` (`self.GetOwner`))))
  (set `self.Physics Body` _asprimitive_component))

(event `Reset`
  (set `self.Force` 0.0))

(fn `Add Force`
  (params (Force :type "Float (double-precision)"))
  (set `self.Force` (+ Force (`self.Force`))))

(fn `Add Torque`
  (params (Torque :type "Float (double-precision)"))
  (`PrimitiveComponent.AddTorqueInDegrees` (`self.Physics Body`) (`KismetMathLibrary.MakeVector` 0.0 0.0 Torque) "None" false))

(fn `Apply Force`
  (`PrimitiveComponent.AddForceAtLocation` (`self.Physics Body`) (* (`self.GetUpVector`) (`self.Force`)) (`self.K2_GetComponentLocation`) "None")
  (set `self.Force` 0.0))